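; BP_Chest is an interactable treasure chest that opens once for a player holding both keys.
; The Interaction event reveals two key meshes and plays a timeline that slides and rotates them into place.
; When that finishes, the Opening timeline, rate-scaled by OpeningTime, rolls the lid by OpeningAngle, brightens four point lights and raises the treasure from transforms cached at BeginPlay.
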(event EventInteraction
  (params (Player :type BP%20First%20Person%20Character%20Object%20Reference))
  (bind _basetreasurelocation (Variables|Default|GetBaseTreasureLocation))
  (bind _basechestrotation (Variables|Default|GetBaseChestRotation))
  ;[0 0 0 0.5] Interact
  (if (and (Variables|/Game/Blueprints/Implemented/BP_FirstPersonCharacter.BP_FirstPersonCharacter_C|GetHasKey1 Player) (Variables|/Game/Blueprints/Implemented/BP_FirstPersonCharacter.BP_FirstPersonCharacter_C|GetHasKey2 Player))
    (Utilities|FlowControl|DoOnce false
      (:Completed
        (Rendering|SetVisibility (Variables|Default|GetKey1) true false)
        (Rendering|SetVisibility (Variables|Default|GetKey2) true false)
        (bind (_direction _rotation _location) (Timeline|Timeline PlayFromStart)
          (:Update
            ;;[0 0.1235 0.15 0.5] Key
            (Transformation|SetRelativeLocation (Variables|Default|GetKey1) (Math|Vector|MakeVector 19.0 (Math|Float|Lerp 1e+02 7e+01 _location) 4.0) false false)
            (Transformation|SetRelativeLocation (Variables|Default|GetKey2) (Math|Vector|MakeVector -19.0 (Math|Float|Lerp 1e+02 7e+01 _location) 4.0) false false)
            (Transformation|SetRelativeRotation (Variables|Default|GetKey1) (Math|Rotator|MakeRotator 0.0 (Math|Float|Lerp -9e+01 0.0 _rotation) 1.8e+02) false false)
            (Transformation|SetRelativeRotation (Variables|Default|GetKey2) (Math|Rotator|MakeRotator 0.0 (Math|Float|Lerp -9e+01 0.0 _rotation) 1.8e+02) false false))
          (:Finished
            ;;[0.15 0.1212 0 0.5] Chest Opening
            (bind _alpha (Timeline|Opening PlayFromStart)
              (:Update
                (Transformation|SetWorldRotation (Variables|Default|GetCHest_Cover) (Math|Rotator|MakeRotator (Math|Float|Lerp (.roll _basechestrotation) (- (.roll _basechestrotation) (Variables|Default|GetOpeningAngle)) _alpha) (.pitch _basechestrotation) (.yaw _basechestrotation)) false false)
                (Rendering|Components|Light|SetIntensity (Variables|Default|GetPointLight) (* _alpha 2e+03))
                (Rendering|Components|Light|SetIntensity (Variables|Default|GetPointLight1) (* _alpha 2e+03))
                (Rendering|Components|Light|SetIntensity (Variables|Default|GetPointLight2) (* _alpha 2e+03))
                (Rendering|Components|Light|SetIntensity (Variables|Default|GetPointLight3) (* _alpha 2e+03))
                (Transformation|SetWorldLocation (Variables|Default|GetTreasure) (Math|Vector|MakeVector (.x _basetreasurelocation) (.y _basetreasurelocation) (Math|Float|Lerp (.z _basetreasurelocation) (+ (.z _basetreasurelocation) 2e+01) _alpha)) false false)))))))))

(event EventBeginPlay
  ;[0.15 0.004139 0.001547 0.5] Begin Play
  (Variables|Default|SetBaseChestRotation (Transformation|GetWorldRotation (Variables|Default|GetCHest_Cover)))
  (Components|Timeline|SetPlayRate (Variables|Default|GetOpening) (/ 1.0 (Variables|Default|GetOpeningTime)))
  (Variables|Default|SetBaseTreasureLocation (Transformation|GetWorldLocation (Variables|Default|GetTreasure))))

(fn ConstructionScript)