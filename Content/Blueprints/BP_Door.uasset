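; Interactable double door that swings both leaves open and closed in opposite yaw directions, or plays a 2D locked sound when locked.
; BeginPlay caches both leaves' starting world rotations and scales the DoorMoving timeline's play rate from the opening time.
; Interaction toggles the Open state and plays the timeline forward or in reverse, lerping yaw by the door angle.
; A busy flag blocks new interactions until the timeline finishes.
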(event EventInteraction
  (params (Player :type BP%20First%20Person%20Character%20Object%20Reference))
  (bind _baserotationleft (Variables|Default|GetBaseRotationLeft))
  (bind _baserotationright (Variables|Default|GetBaseRotationRight))
  ;[0.15 0.15 0.15 0.5] Interact
  (if (Variables|Default|GetIsNotLocked)
    (if (Variables|Default|GetNotOpening)
      (Variables|Default|SetNotOpening false)
      (if (Variables|Default|GetOpen)
        (Variables|Default|SetOpen false)
        ;;[0.01093 0.15 0 0.5] Opening
        (bind _alpha (Timeline|DoorMoving ReverseFromEnd)
          (:Update
            (Transformation|SetWorldRotation (Variables|Default|GetSceneLeft) (Math|Rotator|MakeRotator (.roll _baserotationleft) (.pitch _baserotationleft) (Math|Float|Lerp (.yaw _baserotationleft) (- (.yaw _baserotationleft) (Variables|Default|GetDoorAngle)) _alpha)) false false)
            (Transformation|SetWorldRotation (Variables|Default|GetSceneRight) (Math|Rotator|MakeRotator (.roll _baserotationright) (.pitch _baserotationright) (Math|Float|Lerp (.yaw _baserotationright) (+ (.yaw _baserotationright) (Variables|Default|GetDoorAngle)) _alpha)) false false))
          (:Finished
            (Variables|Default|SetNotOpening true)))
        (else
          (Variables|Default|SetOpen true)
          (Timeline|DoorMoving PlayFromStart))))
    (else
      (Audio|PlaySound2D "/Game/Audio/SFX_LockedDoor.SFX_LockedDoor" 1.0 1.0 0.0 0 0))))

(event EventBeginPlay
  ;[0.6146 0.6146 0.6146 0.5] Begin Play
  (Variables|Default|SetBaseRotationLeft (Transformation|GetWorldRotation (Variables|Default|GetSceneLeft)))
  (Variables|Default|SetBaseRotationRight (Transformation|GetWorldRotation (Variables|Default|GetSceneRight)))
  (Components|Timeline|SetPlayRate (Variables|Default|GetDoorMoving) (/ 1.0 (Variables|Default|GetDoorOpeningTime))))

(fn ConstructionScript)